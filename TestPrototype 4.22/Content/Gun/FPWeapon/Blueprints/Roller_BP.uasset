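; Roller weapon actor owned by a RollerCharacter_BP that damages opposing-team actors on contact and leaves roller decals in the world.
; On overlap, it uses the owner's first tag as the team and sends a fixed health reduction through the IDamege interface to actors lacking that tag.
; The Rolling event spawns a test roller decal at its Box component's transform and creates an unparameterized dynamic material instance on it.
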(event Custom|Rolling
  (bind _box (Variables|Default|GetBox))
  (bind _returnvalue (Rendering|Decal|SpawnDecalatLocation "/Game/Decals/M_TestRollerDecal.M_TestRollerDecal" (Math|Conversions|ToVector(Float) (Variables|Default|GetDecalSize)) (Transformation|GetWorldLocation _box) (Transformation|GetWorldRotation _box) 0.0))
  (Rendering|Material|CreateDynamicMaterialInstance _returnvalue :!class /Script/Engine.DecalComponent))

(event EventBeginPlay)

(event EventTick
  (params (DeltaSeconds :type Float%20%28single-precision%29)))

(event Collision|EventActorBeginOverlap
  (params (OtherActor :type Actor%20Object%20Reference))
  ;[1 1 1] 데미지 입히는곳 , 내 주인이랑 태그가 달라야 데미지 들어가도록
  (bind _asroller_character_bp (Utilities|Casting|CastToRollerCharacter_BP (Components|GetOwner)))
  (if (Utilities|DoesObjectImplementInterface OtherActor "/Game/Characters/UnrealBasicCharacter/iDamege.iDamege_C")
    (if (not (Actor|ActorHasTag OtherActor (Utilities|Array|Get(acopy) (Variables|/Script/Engine.Actor|GetTags _asroller_character_bp))))
      (Class|IDamege|AffectHealth(Message) OtherActor -1e+02 (Utilities|Array|Get(acopy) (Variables|/Script/Engine.Actor|GetTags _asroller_character_bp))))))

(fn ConstructionScript)