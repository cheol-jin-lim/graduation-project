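; Gun projectile actor that damages opposing-team actors and leaves decals where it hits.
; On overlap, it sends a fixed health reduction through the IDamege interface to actors lacking the team tag taken from its owner's owner.
; On a collision hit, it spawns a randomly chosen blue or test decal aligned to the surface normal, then destroys itself.
; The decal's dynamic material "frame" randomization is disconnected and never runs.
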(event OnComponentHit(ProjectileColiision)
  (params (HitComponent :type Primitive%20Component%20Object%20Reference) (OtherActor :type Actor%20Object%20Reference) (OtherComp :type Primitive%20Component%20Object%20Reference) (NormalImpulse :type Vector :default "0, 0, 0") (Hit :type Hit%20Result%20Structure%20%28by%20ref%29))
  (bind _returnvalue (Math|Conversions|RotationFromXVector (.normal Hit)))
  (bind _decalsize (Variables|Default|GetDecalSize))
  (bind _returnvalue_2 (Math|Conversions|ToVector(Float) _decalsize))
  (Variables|Default|SetTraceEnd (.traceend Hit))
  (bind _output_get (Variables|Default|SetBlueAndRed (Math|Random|RandomIntegerinRange 0 1)))
  (if (Math|Conversions|ToBoolean(Integer) _output_get)
    (bind _returnvalue_3 (Rendering|Decal|SpawnDecalatLocation "/Game/Decals/M_BlueDecal.M_BlueDecal" _returnvalue_2 (.location Hit) _returnvalue 0.0))
    (Rendering|Material|CreateDynamicMaterialInstance _returnvalue_3 :!class /Script/Engine.DecalComponent)
    (Actor|DestroyActor self)
    (else
      (bind _returnvalue_4 (Rendering|Decal|SpawnDecalatLocation "/Game/Decals/M_TestDecal.M_TestDecal" _returnvalue_2 (.location Hit) _returnvalue 0.0))
      (bind _returnvalue_5 (Rendering|Material|CreateDynamicMaterialInstance _returnvalue_4 :!class /Script/Engine.DecalComponent))
      (Actor|DestroyActor self))))

(event EventBeginPlay)

(event Collision|EventActorBeginOverlap
  (params (OtherActor :type Actor%20Object%20Reference))
  (bind _returnvalue (Components|GetOwner))
  (bind _returnvalue_2 (Components|GetOwner _returnvalue))
  (bind _tags (Variables|/Script/Engine.Actor|GetTags _returnvalue_2))
  (bind _output (Utilities|Array|Get(acopy) _tags))
  (if (Utilities|DoesObjectImplementInterface OtherActor "/Game/Characters/UnrealBasicCharacter/iDamege.iDamege_C")
    (if (not (Actor|ActorHasTag OtherActor _output))
      (Class|IDamege|AffectHealth(Message) OtherActor -2e+01 _output))))

(event EventTick
  (params (DeltaSeconds :type Float%20%28single-precision%29)))

(fn ConstructionScript)