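; BombProjectile is a projectile that damages opposing-team actors it overlaps and leaves a decal where it hits.
; On overlap, actors implementing IDamege lose a fixed amount of health unless they carry the first tag of the projectile's owner's owner, which serves as the team.
; A collision component hit spawns a decal aligned to the surface normal, creates its dynamic material instance and destroys the projectile.
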(event OnComponentHit(BombProjectileCollision)
  (params (HitComponent :type Primitive%20Component%20Object%20Reference) (OtherActor :type Actor%20Object%20Reference) (OtherComp :type Primitive%20Component%20Object%20Reference) (NormalImpulse :type Vector :default "0, 0, 0") (Hit :type Hit%20Result%20Structure%20%28by%20ref%29))
  (bind _returnvalue (Rendering|Decal|SpawnDecalatLocation "/Game/Decals/M_TestDecal_Inst.M_TestDecal_Inst" (Math|Conversions|ToVector(Float) (Variables|Default|GetDecal%20Size)) (.location Hit) (Math|Conversions|RotationFromXVector (.normal Hit)) 0.0))
  (Rendering|Material|CreateDynamicMaterialInstance _returnvalue :!class /Script/Engine.DecalComponent)
  (Actor|DestroyActor self))

(event EventBeginPlay
  ;[1 1 1] 데미지 입히는곳 , 내 주인이랑 태그가 달라야 데미지 들어가도록
)

(event EventTick
  (params (DeltaSeconds :type Float%20%28single-precision%29))
  ;[1 1 1] 데미지 입히는곳 , 내 주인이랑 태그가 달라야 데미지 들어가도록
)

(event Collision|EventActorBeginOverlap
  (params (OtherActor :type Actor%20Object%20Reference))
  (bind _returnvalue (Components|GetOwner))
  (bind _returnvalue_2 (Components|GetOwner _returnvalue))
  (bind _tags (Variables|/Script/Engine.Actor|GetTags _returnvalue_2))
  (bind _output (Utilities|Array|Get(acopy) _tags))
  ;[1 1 1] 데미지 입히는곳 , 내 주인이랑 태그가 달라야 데미지 들어가도록
  (if (Utilities|DoesObjectImplementInterface OtherActor "/Game/Characters/UnrealBasicCharacter/iDamege.iDamege_C")
    (if (not (Actor|ActorHasTag OtherActor _output))
      (Class|IDamege|AffectHealth(Message) OtherActor -2e+01 _output))))

(fn ConstructionScript)