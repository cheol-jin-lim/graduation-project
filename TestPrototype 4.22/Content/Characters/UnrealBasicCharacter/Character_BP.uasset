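; Player shooter character with movement, look, jump, firing, team-filtered health and timed respawn.
; BeginPlay spawns a weapon onto the mesh's gun socket and registers the character's index and spawn transform in MyGameMode.
; AffectHealth applies deltas from other team tags; at zero health it notifies the game mode, hides character and weapon, then resets at the saved transform after a delay.
; The menu key messages the game mode only in the game level.
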(event EventBeginPlay
  (bind _charactermesh (Variables|Default|GetCharacterMesh))
  (Variables|Default|SetGameLevel "GameScene")
  (Variables|Default|Sethealth 1e+02)
  (Utilities|FlowControl|Sequence
    (:then_0
      (bind _returnvalue (Game|SpawnActorfromClass "/Game/Gun/FPWeapon/Blueprints/Weapon_BP.Weapon_BP_C" (Transformation|GetWorldTransform _charactermesh) "Undefined" self 0))
      (bind _output_get (Variables|Default|SetWeapon _returnvalue))
      (Transformation|AttachComponentToComponent _output_get _charactermesh "GunSocket" "SnapToTarget" "KeepWorld" "KeepRelative" true))
    (:then_1
      (bind _asmy_game_mode (Utilities|Casting|CastToMyGameMode (Game|GetGameMode)))
      ;[1 1 1] 겜 시작하면 내캐릭터 번호 + 위치를 배열로 gamemode에 보내서 저장함
      (bind _output_get_2 (Variables|Default|SetGamemode _asmy_game_mode))
      (bind _output_get_3 (Variables|Default|SetMynum (Variables|/Game/Characters/UnrealBasicCharacter/MyGameMode.MyGameMode_C|GetShooterNum _output_get_2)))
      (Utilities|Array|SetArrayElem (Variables|/Game/Characters/UnrealBasicCharacter/MyGameMode.MyGameMode_C|GetShooterspawnTransform _output_get_2) _output_get_3 (Transformation|GetActorTransform) true)
      (Variables|/Game/Characters/UnrealBasicCharacter/MyGameMode.MyGameMode_C|SetShooterNum _output_get_2 (+ _output_get_3 1)))))

(event Collision|EventActorBeginOverlap
  (params (OtherActor :type Actor%20Object%20Reference)))

(event EventTick
  (params (DeltaSeconds :type Float%20%28single-precision%29)))

(event EventAffectHealth
  (params (Delta :type Float%20%28single-precision%29) (Team :type Name :default "None"))
  ;[1 1 1] 총알이 내 태그랑 달라야 데미지 주도록
  (if (not (Utilities|Name|Equal(Name) Team (Utilities|Array|Get(acopy) (Variables|Actor|GetTags self))))
    ;[1 1 1] 데미지 + 내체력 연산 후 0보다 작은지 판별
    (Variables|Default|Sethealth (+ Delta (Variables|Default|Gethealth)))
    (if (<= (Variables|Default|Gethealth) 0.0)
      ;[1 1 1] 죽었으면 숨기고 충돌끄고 death -1
      (Rendering|SetActorHiddenInGame self true)
      (Collision|SetActorEnableCollision false)
      (Class|IGameover|AffectGame(Message) (Game|GetGameMode) -1)
      ;[1 1 1] 3초뒤에 다시 스폰
      (Utilities|FlowControl|Delay 3.0)
      (Transformation|SetActorTransform self (Utilities|Array|Get(acopy) (Variables|/Game/Characters/UnrealBasicCharacter/MyGameMode.MyGameMode_C|GetShooterspawnTransform (stale EventBeginPlay _output_get_2)) (Variables|Default|GetMynum)))
      (Rendering|SetActorHiddenInGame self false)
      (Collision|SetActorEnableCollision true)
      (Variables|Default|SetHealth 1e+02))))

(event Input|ActionEvents|InputActionJump
  (params (Key :type Key%20Structure))
  ;[1 1 1] 점프 처리
  (:Pressed
    (Character|Jump)))

(event Input|ActionEvents|InputActionFire
  (params (Key :type Key%20Structure))
  (:Pressed
    (Default|Fire (Variables|Default|GetWeapon))))

(event Input|ActionEvents|InputActionMenuOpen
  (params (Key :type Key%20Structure))
  (:Pressed
    (bind _returnvalue (Game|GetCurrentLevelName true))
    (if (Utilities|Enum|Equal(Enum) _returnvalue (Variables|Default|GetGameLevel))
      (Class|IMenu|IMenu(Message) (Game|GetGameMode)))))

(event Input|AxisEvents|InputAxisMoveForward
  (params (AxisValue :type Float%20%28single-precision%29))
  ;[1 1 1] 캐릭터 movement
  (Pawn|Input|AddMovementInput (Math|Vector|GetForwardVector (Math|Rotator|MakeRotator 0.0 0.0 (.Yaw (Math|Rotator|BreakRotator (Pawn|GetControlRotation :!class /Script/Engine.Pawn))))) AxisValue false))

(event Input|AxisEvents|InputAxisMoveRight
  (params (AxisValue :type Float%20%28single-precision%29))
  ;[1 1 1] 캐릭터 movement
  (Pawn|Input|AddMovementInput (Math|Vector|GetRightVector (Math|Rotator|MakeRotator 0.0 0.0 (.Yaw (Math|Rotator|BreakRotator (Pawn|GetControlRotation :!class /Script/Engine.Pawn))))) AxisValue false))

(event Input|AxisEvents|InputAxisTurn
  (params (AxisValue :type Float%20%28single-precision%29))
  ;[1 1 1] 마우스 Input처리
  (Pawn|Input|AddControllerYawInput AxisValue))

(event Input|AxisEvents|InputAxisLookUp
  (params (AxisValue :type Float%20%28single-precision%29))
  ;[1 1 1] 마우스 Input처리
  (Pawn|Input|AddControllerPitchInput AxisValue))

(fn ConstructionScript)