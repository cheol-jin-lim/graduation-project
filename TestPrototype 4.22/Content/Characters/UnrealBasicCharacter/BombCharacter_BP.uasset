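; Player character that carries a bomb weapon, with movement, look, jump and fire input, team-filtered health and respawning.
; On BeginPlay it attaches a spawned BombWeapon_BP to BombSocket and registers its index and spawn transform with MyGameMode.
; AffectHealth adds deltas from other teams, identified by the first actor tag.
; At zero health it passes index, tags and material to BombRespawn for restoration through RespawnOption, then destroys itself and its weapon.
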(event EventBeginPlay
  (bind _charactermesh (Variables|Default|GetCharacterMesh))
  (Utilities|FlowControl|Sequence
    (:then_0
      (Variables|Default|SetHealth 1e+02)
      (bind _returnvalue (Game|SpawnActorfromClass "/Game/Gun/FPWeapon/Blueprints/BombWeapon_BP.BombWeapon_BP_C" (Transformation|GetWorldTransform _charactermesh) "Undefined" self 0))
      (bind _output_get (Variables|Default|SetWeapon _returnvalue))
      (Transformation|AttachComponentToComponent _output_get _charactermesh "BombSocket" "SnapToTarget" "KeepWorld" "KeepRelative" true))
    (:then_1
      ;[1 1 1] my game mode에 내 캐릭터 번호(몇번째인지) 랑 내 스폰 위치를 넘겨줌 // 리스폰할때 그곳에서 그대로 리스폰 하려고
      (bind _asmy_game_mode (Utilities|Casting|CastToMyGameMode (Game|GetGameMode)))
      (bind _output_get_2 (Variables|Default|SetMode _asmy_game_mode))
      (bind _output_get_3 (Variables|Default|SetMynum (Variables|/Game/Characters/UnrealBasicCharacter/MyGameMode.MyGameMode_C|GetBombNum _output_get_2)))
      (Utilities|Array|SetArrayElem (Variables|/Game/Characters/UnrealBasicCharacter/MyGameMode.MyGameMode_C|GetBombSpawnTransform _output_get_2) _output_get_3 (Transformation|GetActorTransform) true)
      (Variables|/Game/Characters/UnrealBasicCharacter/MyGameMode.MyGameMode_C|SetBombNum _output_get_2 (+ _output_get_3 1)))))

(event Collision|EventActorBeginOverlap
  (params (OtherActor :type Actor%20Object%20Reference)))

(event EventTick
  (params (DeltaSeconds :type Float%20%28single-precision%29)))

(event EventRespawnOption
  (params (Tag :type Array%20of%20Names) (mater :type Material%20Interface%20Object%20Reference))
  ;[1 1 1] my game mode에서 리스폰 할때 부름. 태그 메쉬 셋
  (Variables|Default|SetTags Tag)
  (Rendering|Material|SetMaterial (Variables|Default|GetCharacterMesh) 0 mater))

(event EventAffectHealth
  (params (Delta :type Float%20%28single-precision%29) (Team :type Name :default "None"))
  ;[1 1 1] 코데미지 들어오면 내 피랑 데미지랑 합치는 곳
  (if (not (Utilities|Name|Equal(Name) Team (Utilities|Array|Get(acopy) (Variables|Actor|GetTags self))))
    (bind _output_get (Variables|Default|Sethealth (+ Delta (Variables|Default|Gethealth))))
    (Development|PrintString (Utilities|String|ToString(Float) _output_get))
    (if (<= (Variables|Default|Gethealth) 0.0)
      ;[1 1 1] 리스폰, 리스폰 될때 태그,메쉬 넘겨주는곳 그대로 리스폰 하려고
      (bind _asmy_game_mode (Utilities|Casting|CastToMyGameMode (Game|GetGameMode)))
      (Default|BombRespawn _asmy_game_mode (Variables|Default|GetMynum) (Variables|Actor|GetTags) (Rendering|Material|GetMaterial (Variables|Default|GetCharacterMesh) 0))
      (Actor|DestroyActor (Variables|Default|GetWeapon))
      (Class|IGameover|AffectGame(Message) (Game|GetGameMode) -1))))

(event Input|ActionEvents|InputActionJump
  (params (Key :type Key%20Structure))
  ;[1 1 1] 점프 처리
  (:Pressed
    (Character|Jump)))

(event Input|ActionEvents|InputActionFire
  (params (Key :type Key%20Structure))
  (:Pressed
    (Default|Fire (Variables|Default|GetWeapon))))

(event Input|AxisEvents|InputAxisMoveForward
  (params (AxisValue :type Float%20%28single-precision%29))
  ;[1 1 1] 캐릭터 movement
  (Pawn|Input|AddMovementInput (Math|Vector|GetForwardVector (Math|Rotator|MakeRotator 0.0 0.0 (.Yaw (Math|Rotator|BreakRotator (Pawn|GetControlRotation :!class /Script/Engine.Pawn))))) AxisValue false))

(event Input|AxisEvents|InputAxisMoveRight
  (params (AxisValue :type Float%20%28single-precision%29))
  ;[1 1 1] 캐릭터 movement
  (Pawn|Input|AddMovementInput (Math|Vector|GetRightVector (Math|Rotator|MakeRotator 0.0 0.0 (.Yaw (Math|Rotator|BreakRotator (Pawn|GetControlRotation :!class /Script/Engine.Pawn))))) AxisValue false))

(event Input|AxisEvents|InputAxisTurn
  (params (AxisValue :type Float%20%28single-precision%29))
  ;[1 1 1] 마우스 Input처리
  (Pawn|Input|AddControllerYawInput AxisValue))

(event Input|AxisEvents|InputAxisLookUp
  (params (AxisValue :type Float%20%28single-precision%29))
  ;[1 1 1] 마우스 Input처리
  (Pawn|Input|AddControllerPitchInput AxisValue))

(fn ConstructionScript)