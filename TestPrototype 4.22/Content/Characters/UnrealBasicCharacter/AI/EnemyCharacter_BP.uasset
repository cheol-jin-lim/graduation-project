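; EnemyCharacter_BP is a character Blueprint in the AI folder that carries a gun, though its graph holds player input handling and no AI logic.
; Axis inputs drive movement relative to control yaw and mouse look, and an action input triggers jumping.
; BeginPlay spawns a Weapon_BP and attaches it to the mesh's GunSocket.
; The Fire input calls that weapon's Fire and prints a debug string.
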(event EventBeginPlay
  (bind _mesh (Variables|Character|GetMesh))
  (Utilities|FlowControl|Sequence
    (:then_0
      (bind _returnvalue (Game|SpawnActorfromClass "/Game/Gun/FPWeapon/Blueprints/Weapon_BP.Weapon_BP_C" (Transformation|GetWorldTransform _mesh) "Undefined" 0 0))
      (bind _output_get (Variables|Default|SetWeapon _returnvalue))
      (Transformation|AttachComponentToComponent _output_get _mesh "GunSocket" "SnapToTarget" "KeepWorld" "KeepRelative" true))))

(event Collision|EventActorBeginOverlap
  (params (OtherActor :type Actor%20Object%20Reference)))

(event EventTick
  (params (DeltaSeconds :type Float%20%28single-precision%29)))

(event Input|ActionEvents|InputActionJump
  (params (Key :type Key%20Structure))
  ;[1 1 1] 점프 처리
  (:Pressed
    (Character|Jump)))

(event Input|ActionEvents|InputActionFire
  (params (Key :type Key%20Structure))
  (:Pressed
    (Default|Fire (Variables|Default|GetWeapon))
    (Development|PrintString "Hello")))

(event Input|AxisEvents|InputAxisMoveForward
  (params (AxisValue :type Float%20%28single-precision%29))
  ;[1 1 1] 캐릭터 movement
  (Pawn|Input|AddMovementInput (Math|Vector|GetForwardVector (Math|Rotator|MakeRotator 0.0 0.0 (.Yaw (Math|Rotator|BreakRotator (Pawn|GetControlRotation :!class /Script/Engine.Pawn))))) AxisValue false))

(event Input|AxisEvents|InputAxisMoveRight
  (params (AxisValue :type Float%20%28single-precision%29))
  ;[1 1 1] 캐릭터 movement
  (Pawn|Input|AddMovementInput (Math|Vector|GetRightVector (Math|Rotator|MakeRotator 0.0 0.0 (.Yaw (Math|Rotator|BreakRotator (Pawn|GetControlRotation :!class /Script/Engine.Pawn))))) AxisValue false))

(event Input|AxisEvents|InputAxisTurn
  (params (AxisValue :type Float%20%28single-precision%29))
  ;[1 1 1] 마우스 Input처리
  (Pawn|Input|AddControllerYawInput AxisValue))

(event Input|AxisEvents|InputAxisLookUp
  (params (AxisValue :type Float%20%28single-precision%29))
  ;[1 1 1] 마우스 Input처리
  (Pawn|Input|AddControllerPitchInput AxisValue))

(fn ConstructionScript)