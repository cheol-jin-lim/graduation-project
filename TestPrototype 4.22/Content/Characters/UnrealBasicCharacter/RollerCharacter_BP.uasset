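; Playable roller character with team-based health, movement, mouse look and jumping.
; On BeginPlay it spawns a Roller_BP weapon on its mesh socket and registers its spawn transform with MyGameMode under its own index.
; Holding RollerDown calls the weapon's Rolling every tick.
; Other-team health changes can kill it: it asks the game mode to respawn it with the same tags and material, then destroys itself and the weapon.
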(event EventBeginPlay
  (bind _charactermesh (Variables|Default|GetCharacterMesh))
  (Variables|Default|SetHealth 1e+02)
  (Utilities|FlowControl|Sequence
    (:then_0
      (bind _returnvalue (Utilities|NewMacro0 (Transformation|GetWorldTransform _charactermesh) self))
      (bind _output_get (Variables|Default|SetWeapon _returnvalue))
      (Transformation|AttachComponentToComponent _output_get _charactermesh "RollerSocket" "SnapToTarget" "KeepWorld" "KeepRelative" true))
    (:then_1
      (bind _asmy_game_mode (Utilities|Casting|CastToMyGameMode (Game|GetGameMode)))
      (bind _output_get_2 (Variables|Default|SetGamemode _asmy_game_mode))
      (bind _output_get_3 (Variables|Default|SetMynum (Variables|/Game/Characters/UnrealBasicCharacter/MyGameMode.MyGameMode_C|GetRollerNum _output_get_2)))
      (Utilities|Array|SetArrayElem (Variables|/Game/Characters/UnrealBasicCharacter/MyGameMode.MyGameMode_C|GetRollerspawnTransform _output_get_2) _output_get_3 (Transformation|GetActorTransform) true)
      (Variables|/Game/Characters/UnrealBasicCharacter/MyGameMode.MyGameMode_C|SetRollerNum _output_get_2 (+ (Variables|/Game/Characters/UnrealBasicCharacter/MyGameMode.MyGameMode_C|GetRollerNum _output_get_2) 1)))))

(event Collision|EventActorBeginOverlap
  (params (OtherActor :type Actor%20Object%20Reference)))

(event EventRespawnOption
  (params (Tag :type Array%20of%20Names) (mater :type Material%20Interface%20Object%20Reference))
  (Variables|Default|SetTags Tag)
  (Rendering|Material|SetMaterial (Variables|Default|GetCharacterMesh) 0 mater))

(event EventTick
  (params (DeltaSeconds :type Float%20%28single-precision%29))
  (if (Variables|Default|GetIsRolling?)
    (Default|Rolling (Variables|Default|GetWeapon))))

(event EventAffectHealth
  (params (Delta :type Float%20%28single-precision%29) (Team :type Name :default "None"))
  (if (not (Utilities|Name|Equal(Name) Team (Utilities|Array|Get(acopy) (Variables|Actor|GetTags self))))
    (bind _output_get (Variables|Default|Sethealth (+ Delta (Variables|Default|Gethealth))))
    (Development|PrintString (Utilities|String|ToString(Float) _output_get))
    (if (<= (Variables|Default|Gethealth) 0.0)
      (bind _asmy_game_mode (Utilities|Casting|CastToMyGameMode (Game|GetGameMode)))
      (Default|RollerRespawn _asmy_game_mode (Variables|Default|GetMynum) (Variables|Actor|GetTags self) (Rendering|Material|GetMaterial (Variables|Default|GetCharacterMesh) 0))
      (Actor|DestroyActor (Variables|Default|GetWeapon))
      (Class|IGameover|AffectGame(Message) (Game|GetGameMode) -1))))

(event Input|ActionEvents|InputActionJump
  (params (Key :type Key%20Structure))
  ;[1 1 1] 점프 처리
  (:Pressed
    (Character|Jump)))

(event Input|ActionEvents|InputActionFire
  (params (Key :type Key%20Structure)))

(event Input|ActionEvents|InputActionRollerDown
  (params (Key :type Key%20Structure))
  (:Pressed
    (Variables|Default|SetIsRolling? true))
  (:Released
    (Variables|Default|SetIsRolling? false)))

(event Input|AxisEvents|InputAxisMoveForward
  (params (AxisValue :type Float%20%28single-precision%29))
  ;[1 1 1] 캐릭터 movement
  (Pawn|Input|AddMovementInput (Math|Vector|GetForwardVector (Math|Rotator|MakeRotator 0.0 0.0 (.Yaw (Math|Rotator|BreakRotator (Pawn|GetControlRotation :!class /Script/Engine.Pawn))))) AxisValue false))

(event Input|AxisEvents|InputAxisMoveRight
  (params (AxisValue :type Float%20%28single-precision%29))
  ;[1 1 1] 캐릭터 movement
  (Pawn|Input|AddMovementInput (Math|Vector|GetRightVector (Math|Rotator|MakeRotator 0.0 0.0 (.Yaw (Math|Rotator|BreakRotator (Pawn|GetControlRotation :!class /Script/Engine.Pawn))))) AxisValue false))

(event Input|AxisEvents|InputAxisTurn
  (params (AxisValue :type Float%20%28single-precision%29))
  ;[1 1 1] 마우스 Input처리
  (Pawn|Input|AddControllerYawInput AxisValue))

(event Input|AxisEvents|InputAxisLookUp
  (params (AxisValue :type Float%20%28single-precision%29))
  ;[1 1 1] 마우스 Input처리
  (Pawn|Input|AddControllerPitchInput AxisValue))

(fn ConstructionScript)